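; BP_Key is an interactable key pickup actor that the player collects to affect a linked door.
; Interaction notifies the referenced door through PickUpKeyMessage, plays a pickup sound, destroys the key and prints a debug pickup message.
; It always reports itself as interactable and caches the player's BaseCharacter on BeginPlay, though the interaction logic does not use that reference.
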(event EventBeginPlay
  (bind _asbase_character (Utilities|Casting|CastToBaseCharacter (Game|GetPlayerCharacter 0)))
  (Variables|Default|SetCharacterReference _asbase_character))

(event Collision|EventActorBeginOverlap
  (params (OtherActor :type Actor%20Object%20Reference)))

(event EventTick
  (params (DeltaSeconds :type Float%20%28single-precision%29)))

(event EventOnInteract
  (params (Interacting%20Player :type Base%20Character%20Object%20Reference))
  (Class|BPIPickUpKey|PickUpKey(Message) (Variables|Default|GetBP_Door))
  (Audio|PlaySound2D "/Game/Audio/KeyPickup.KeyPickup" 1.0 1.0 0.0 0 0)
  (Actor|DestroyActor)
  (Development|PrintString "+ Key" true true "(R=1.000000,G=0.000000,B=0.657874,A=1.000000)"))

(fn ConstructionScript)

(fn IsInteractable
  (return true))