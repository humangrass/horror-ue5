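; Interactable door actor that swings open and closed, with an optional lock that requires a key.
; OnInteract checks the lock and key flag, then plays or reverses a timeline whose track directly sets the pivot's relative yaw.
; PickUpKey sets the key flag on the door itself; a locked door without it only prints a message.
; BeginPlay caches the player character, though these graphs never use it.
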(event EventBeginPlay
  (bind _asbase_character (Utilities|Casting|CastToBaseCharacter (Game|GetPlayerCharacter 0)))
  (Variables|Default|SetCharacterReference _asbase_character))

(event Collision|EventActorBeginOverlap
  (params (OtherActor :type Actor%20Object%20Reference)))

(event EventTick
  (params (DeltaSeconds :type Float%20%28single-precision%29)))

(event EventOnInteract
  (params (Interacting%20Player :type Base%20Character%20Object%20Reference))
  (bind _pivotpoint (Variables|Default|GetPivotPoint))
  (bind _relativerotation (Variables|/Script/Engine.SceneComponent|GetRelativeRotation _pivotpoint))
  ;[0.15 0.15 0.15 0.5] Close/Open Door
  (if (Variables|Default|GetIsDoorLocked)
    (if (Variables|Default|GetIsPlayerHasKey)
      (if (Variables|Default|GetIsDoorClosed)
        (Variables|Default|SetIsDoorClosed false :!label _label)
        (bind _alpha (Timeline|Open/CloseDoor Play)
          (:Update
            (Transformation|SetRelativeRotation _pivotpoint (Math|Rotator|MakeRotator (.roll _relativerotation) (.pitch _relativerotation) _alpha) false false)))
        (else
          (Variables|Default|SetIsDoorClosed true :!label _label_2)
          (Timeline|Open/CloseDoor Reverse)))
      (else
        (Development|PrintString "You need a right key")))
    (elif (Variables|Default|GetIsDoorClosed)
      (goto _label)
      (else
        (goto _label_2)))))

(event EventPickUpKey
  (Variables|Default|SetIsPlayerHasKey true))

(fn ConstructionScript)

(fn IsInteractable
  (return true))