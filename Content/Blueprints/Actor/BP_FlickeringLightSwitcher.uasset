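; Interactable wall-switch style actor that toggles the visibility of a referenced Light's root component and plays a click sound.
; OnInteract plays or reverses a timeline that slides the Trigger component along Y to match the toggle.
; BeginPlay caches the player character and positions Trigger from IsLightON, with X and Z swapped in the true branch.
; IsLightON is set true when the light is hidden, opposite to its name.
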(event EventBeginPlay
  (bind _trigger (Variables|Default|GetTrigger))
  (bind _relativelocation (Variables|/Script/Engine.SceneComponent|GetRelativeLocation _trigger))
  (bind _asbase_character (Utilities|Casting|CastToBaseCharacter (Game|GetPlayerCharacter 0)))
  (Variables|Default|SetCharacterReference _asbase_character)
  ;[0.15 0.15 0.15 0.5] Корректная позиция переключателя при старте сцены
  (if (Variables|Default|GetIsLightON)
    (Transformation|SetRelativeLocation _trigger (Math|Vector|MakeVector (.z _relativelocation) 35.0 (.x _relativelocation)) false false)
    (else
      (Transformation|SetRelativeLocation _trigger (Math|Vector|MakeVector (.x _relativelocation) 75.0 (.z _relativelocation)) false false))))

(event Collision|EventActorBeginOverlap
  (params (OtherActor :type Actor%20Object%20Reference)))

(event EventTick
  (params (DeltaSeconds :type Float%20%28single-precision%29)))

(event EventOnInteract
  (params (Interacting%20Player :type Base%20Character%20Object%20Reference))
  (bind _light (Variables|Default|GetLight))
  (bind _trigger (Variables|Default|GetTrigger))
  (bind _relativelocation (Variables|/Script/Engine.SceneComponent|GetRelativeLocation _trigger))
  (bind _rootcomponent (Variables|/Script/Engine.Actor|GetRootComponent _light))
  (Audio|PlaySound2D "/Game/Audio/Flashlight_Switch.Flashlight_Switch" 1.0 1.0 0.0 0 0)
  (if (Rendering|IsVisible _rootcomponent)
    (Rendering|SetVisibility _rootcomponent false false)
    (Variables|Default|SetIsLightON true)
    (bind _turnonoff (Timeline|OnOff%20Timeline Play)
      (:Update
        (Transformation|SetRelativeLocation _trigger (Math|Vector|MakeVector (.x _relativelocation) _turnonoff (.z _relativelocation)) false false)))
    (else
      (Rendering|SetVisibility _rootcomponent true false)
      (Variables|Default|SetIsLightON false)
      (Timeline|OnOff%20Timeline Reverse))))

(fn ConstructionScript)

(fn IsInteractable
  (return true))